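; Showcase variant of the East Ka-52 helicopter that exposes its adjustable parts to generic checkbox, slider and twin-slider controls.
; Each control event forwards its values to setters for damage, rotors, rudder, lights, canopy, cannon, sensor, landing gear and dust plume.
; One twin-slider value drives both rear wheels together.
; Construction defers to the parent, and the BeginPlay, overlap and Tick events are disabled stubs.
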(event `/Game/VigilanteContent/Shared/Blueprints/Showcase/Interfaces/BP_ShowcaseControlsInterface.SetCheckboxVariable0`
  (params (NewState :type Boolean))
  (`self.SetShowDamaged` NewState))

(event `/Game/VigilanteContent/Shared/Blueprints/Showcase/Interfaces/BP_ShowcaseControlsInterface.SetSliderVariable0`
  (params (NewValue :type "Float (double-precision)"))
  (`self.SetRotorSpeed` NewValue))

(event `/Game/VigilanteContent/Shared/Blueprints/Showcase/Interfaces/BP_ShowcaseControlsInterface.SetSliderVariable1`
  (params (NewValue :type "Float (double-precision)"))
  (`self.SetRudder` NewValue))

(event `/Game/VigilanteContent/Shared/Blueprints/Showcase/Interfaces/BP_ShowcaseControlsInterface.SetSliderVariable2`
  (params (NewValue :type "Float (double-precision)"))
  (`self.SetLightsEmissivity` NewValue))

(event `/Game/VigilanteContent/Shared/Blueprints/Showcase/Interfaces/BP_ShowcaseControlsInterface.SetTwinSliderVariable0`
  (params (`bFirstSlider?` :type Boolean) (NewFirstValue :type "Float (double-precision)") (NewSecondValue :type "Float (double-precision)"))
  (`self.SetBottomRotorBlades` NewFirstValue)
  (`self.SetTopRotorBlades` NewSecondValue))

(event `/Game/VigilanteContent/Shared/Blueprints/Showcase/Interfaces/BP_ShowcaseControlsInterface.SetTwinSliderVariable1`
  (params (`bFirstSlider?` :type Boolean) (NewFirstValue :type "Float (double-precision)") (NewSecondValue :type "Float (double-precision)"))
  (`self.SetRotorPitch` NewFirstValue)
  (`self.SetRotorRoll` NewSecondValue))

(event `/Game/VigilanteContent/Shared/Blueprints/Showcase/Interfaces/BP_ShowcaseControlsInterface.SetTwinSliderVariable2`
  (params (`bFirstSlider?` :type Boolean) (NewFirstValue :type "Float (double-precision)") (NewSecondValue :type "Float (double-precision)"))
  (`self.SetCanopyRight` NewFirstValue)
  (`self.SetCanopyLeft` NewSecondValue))

(event `/Game/VigilanteContent/Shared/Blueprints/Showcase/Interfaces/BP_ShowcaseControlsInterface.SetTwinSliderVariable3`
  (params (`bFirstSlider?` :type Boolean) (NewFirstValue :type "Float (double-precision)") (NewSecondValue :type "Float (double-precision)"))
  (`self.SetCannonYaw` NewFirstValue)
  (`self.SetCannonPitch` NewSecondValue))

(event `/Game/VigilanteContent/Shared/Blueprints/Showcase/Interfaces/BP_ShowcaseControlsInterface.SetTwinSliderVariable4`
  (params (`bFirstSlider?` :type Boolean) (NewFirstValue :type "Float (double-precision)") (NewSecondValue :type "Float (double-precision)"))
  (`self.SetSensorYaw` NewFirstValue)
  (`self.SetSensorPitch` NewSecondValue))

(event `/Game/VigilanteContent/Shared/Blueprints/Showcase/Interfaces/BP_ShowcaseControlsInterface.SetTwinSliderVariable5`
  (params (`bFirstSlider?` :type Boolean) (NewFirstValue :type "Float (double-precision)") (NewSecondValue :type "Float (double-precision)"))
  (`self.RectractFrontWheel` NewFirstValue)
  (`self.RetractRearLWheel` NewSecondValue)
  (`self.RetractRearRWheel` NewSecondValue))

(event `/Game/VigilanteContent/Shared/Blueprints/Showcase/Interfaces/BP_ShowcaseControlsInterface.SetCheckboxVariable1`
  (params (NewState :type Boolean))
  (`self.ShowDustPlume` NewState))

(fn `UserConstructionScript`
  (`parent.UserConstructionScript`))